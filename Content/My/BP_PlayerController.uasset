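; Player controller that adds the default Enhanced Input mapping and drives movement of the player character.
; On BeginPlay it casts the player pawn to BP_Player, caching it and its CharacterMovement, then registers IMC_Default.
; IA_Move feeds its Y and X values into AddMovementInput along forward and right vectors from control rotation.
; Forward uses yaw only, while right also includes roll.
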(event `self.ReceiveBeginPlay`
  (`|ExecutionSequence`
    (:`then_0`
      (bind _asbp_player (cast `/Game/My/BP_Player` (`GameplayStatics.GetPlayerPawn` 0)))
      (bind _output_get (set `self.As BP Player` _asbp_player))
      (set `self.Character Movement` (`Character.CharacterMovement` _output_get)))
    (:`then_1`
      (`EnhancedInputSubsystemInterface.AddMappingContext` (subsystem `EnhancedInputLocalPlayerSubsystem`) "/Game/My/MyInput/IMC_Default.IMC_Default" 0 (struct)))))

(event `EnhancedInput|/Game/My/MyInput/IA_Move`
  (params (ActionValue :type "Vector2D Structure") (ElapsedSeconds :type "Float (double-precision)") (TriggeredSeconds :type "Float (double-precision)") (InputAction :type "InputAction Object Reference" :default "/Game/My/MyInput/IA_Move.IA_Move"))
  (bind (_returnvalue_roll _returnvalue_pitch _returnvalue_yaw) (`KismetMathLibrary.BreakRotator` (`Pawn.GetControlRotation` (`self.As BP Player`))))
  (bind (_returnvalue_roll_2 _returnvalue_pitch_2 _returnvalue_yaw_2) (`KismetMathLibrary.BreakRotator` (`Pawn.GetControlRotation` (`self.As BP Player`))))
  (:`Triggered`
    (`|ExecutionSequence`
      (:`then_0`
        (`Pawn.AddMovementInput` (`self.As BP Player`) (`KismetMathLibrary.GetForwardVector` (`KismetMathLibrary.MakeRotator` 0.0 0.0 _returnvalue_yaw_2)) ActionValue_Y false))
      (:`then_1`
        (`Pawn.AddMovementInput` (`self.As BP Player`) (`KismetMathLibrary.GetRightVector` (`KismetMathLibrary.MakeRotator` _returnvalue_roll 0.0 _returnvalue_yaw)) ActionValue_X false)))))

(fn `UserConstructionScript`)